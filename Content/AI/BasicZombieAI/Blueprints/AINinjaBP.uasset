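; Ninja enemy AI that walks to the restaurant door and damages it.
; On BeginPlay it caches the LevelDatabaseActor and player, then uses AIMoveTo toward the database's door.
; Overlapping the door starts a looping, Delay-paced damage cycle that toggles IsDamaged and calls the door's FDamageTrigger.
; Tick calls IsLoS, a stub returning false with unwired look-direction checks; FDamage is empty.
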(event EventBeginPlay
  ;[1 1 1] CastToDatabase
  (bind _outactors (Actor|GetAllActorsOfClass "/Game/Database/LevelDatabaseActor.LevelDatabaseActor_C"))
  (bind _output_get (Variables|Default|SetLevelDatabase (Utilities|Array|Get(acopy) _outactors)))
  (Variables|Default|SetPlayer (Variables|/Game/Database/LevelDatabaseActor.LevelDatabaseActor_C|GetSushiSlasher _output_get))
  ;[1 1 1] BasicMoveToDoor
  (AI|AIMoveTo self "0, 0, 0" (Variables|/Game/Database/LevelDatabaseActor.LevelDatabaseActor_C|GetRestaurantDoor (Variables|Default|GetLevelDatabase)) 3e+01 false))

(event Collision|EventActorBeginOverlap
  (params (OtherActor :type Actor%20Object%20Reference))
  (bind _leveldatabase (Variables|Default|GetLevelDatabase))
  (bind _restaurantdoor (Variables|/Game/Database/LevelDatabaseActor.LevelDatabaseActor_C|GetRestaurantDoor _leveldatabase))
  ;[1 1 1] OverlapDamageDoor
  (if (== OtherActor _restaurantdoor) :!label _label
    (Variables|/Game/Triggers+EventItems/RestaurantDoor.RestaurantDoor_C|SetIsDamaged _restaurantdoor true)
    (Variables|/Game/Triggers+EventItems/RestaurantDoor.RestaurantDoor_C|SetInputDamage _restaurantdoor 2.5) ; DamageToDoor
    (Default|FDamageTrigger _restaurantdoor)
    (Utilities|FlowControl|Delay 1.0) ; DamageRate
  )
  (Variables|/Game/Triggers+EventItems/RestaurantDoor.RestaurantDoor_C|SetIsDamaged _restaurantdoor false)
  (goto _label))

(event EventTick
  (params (DeltaSeconds :type Float%20%28single-precision%29))
  (CallFunction|IsLoS))

(fn ConstructionScript)

(fn IsLoS
  (params (NinjaActor :type AI%20Ninja%20BP%20Object%20Reference))
  (return false))

(fn FDamage)